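; BP_Player is the player pawn, translating axis inputs into movement and view rotation.
; Forward and Stroll move it horizontally along the X/Y components of the control rotation's forward and right vectors, while Zoom follows the full forward vector, including pitch.
; Turn and LookUp feed controller yaw and pitch directly, and Rotate adds yaw scaled by RotationModifier.
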(event EventBeginPlay)

(event Collision|EventActorBeginOverlap
  (params (OtherActor :type Actor%20Object%20Reference)))

(event EventTick
  (params (DeltaSeconds :type Float%20%28single-precision%29)))

(event Input|AxisEvents|InputAxisForward
  (params (AxisValue :type Float%20%28single-precision%29))
  (bind _returnvalue (Game|GetPlayerController 0))
  (bind _returnvalue_2 (Pawn|GetControlRotation _returnvalue :!class /Script/Engine.Controller))
  (bind _returnvalue_3 (Math|Vector|GetForwardVector _returnvalue_2))
  (Pawn|Input|AddMovementInput (Math|Vector|MakeVector (.x _returnvalue_3) (.y _returnvalue_3) 0.0) AxisValue false))

(event Input|AxisEvents|InputAxisStroll
  (params (AxisValue :type Float%20%28single-precision%29))
  (bind _returnvalue (Game|GetPlayerController 0))
  (bind _returnvalue_2 (Pawn|GetControlRotation _returnvalue :!class /Script/Engine.Controller))
  (bind _returnvalue_3 (Math|Vector|GetRightVector _returnvalue_2))
  (Pawn|Input|AddMovementInput (Math|Vector|MakeVector (.x _returnvalue_3) (.y _returnvalue_3) 0.0) AxisValue false))

(event Input|AxisEvents|InputAxisRotate
  (params (AxisValue :type Float%20%28single-precision%29))
  (Pawn|Input|AddControllerYawInput (* (Variables|Default|GetRotationModifier) AxisValue)))

(event Input|AxisEvents|InputAxisTurn
  (params (AxisValue :type Float%20%28single-precision%29))
  (Pawn|Input|AddControllerYawInput AxisValue))

(event Input|AxisEvents|InputAxisLookUp
  (params (AxisValue :type Float%20%28single-precision%29))
  (Pawn|Input|AddControllerPitchInput AxisValue))

(event Input|AxisEvents|InputAxisZoom
  (params (AxisValue :type Float%20%28single-precision%29))
  (Pawn|Input|AddMovementInput (Math|Vector|GetForwardVector (Pawn|GetControlRotation (Game|GetPlayerController 0) :!class /Script/Engine.Controller)) AxisValue false))

(fn ConstructionScript)