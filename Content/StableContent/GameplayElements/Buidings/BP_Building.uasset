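; Placeable building actor that the player moves through the construction manager, with its base price credited back when stopping a move fails.
; Setting its info spawns a child BuildingActor, whose overlaps it forwards for processing and whose emissive color it tints for normal, available or forbidden states.
; Right-clicking an idle building shows a widget-component context menu at the deprojected cursor location; left-click release stops moving and hides it.
; It also creates building details widgets.
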(event Custom|OnBeginChildOverlap
  (params (OverlappedActor :type Actor%20Object%20Reference) (OtherActor :type Actor%20Object%20Reference))
  (Class|ConstructableBuilding|ProcessActorBeginOverlap OtherActor))

(event Custom|StartMoving
  (bind _constructionmanager (CallFunction|GetConstructionManager))
  (Class|ConstructionManager|MoveBuilding _constructionmanager self))

(event Custom|CreateBuilding
  (bind _returnvalue (Class|ConstructableBuilding|CreateBuildingChild))
  (bind _asbuilding_actor (Utilities|Casting|CastToBuildingActor _returnvalue))
  (bind _output_get (Variables|Default|SetBuildingActor _asbuilding_actor))
  (Collision|BindEventtoOnActorBeginOverlap _output_get (delegate Custom|OnBeginChildOverlap))
  (Collision|BindEventtoOnActorEndOverlap _output_get (delegate Custom|OnEndChildOverlap)))

(event Custom|OnEndChildOverlap
  (params (OverlappedActor :type Actor%20Object%20Reference) (OtherActor :type Actor%20Object%20Reference))
  (Class|ConstructableBuilding|ProcessActorEndOverlap OtherActor))

(event EventSetColor
  (params (Material :type BuildingColor%20Enum%20%28by%20ref%29 :default "Color_Normal"))
  (switch Utilities|FlowControl|Switch|SwitchonBuildingColor Material
    (:Color_Normal
      (Variables|Default|SetBuildingEmitColor ""))
    (:Color_Available
      (Variables|Default|SetBuildingEmitColor "(R=0.000000,G=0.100000,B=0.000000,A=1.000000)"))
    (:Color_Inavailable
      (Variables|Default|SetBuildingEmitColor "(R=0.100000,G=0.000000,B=0.000000,A=1.000000)")))
  (Default|SetBuildingColor (Variables|Default|GetBuildingActor) (Variables|Default|GetBuildingEmitColor)))

(fn ConstructionScript)

(fn ChangeState
  (params (newState :type Byte :default 0)))

(fn HideContextMenu
  (bind _ascontext_menu_bp (CallFunction|GetContextMenu))
  (Default|OnHidden _ascontext_menu_bp)
  (Variables|Default|SetWidgetShown false)
  (Collision|SetCollisionEnabled (Variables|Default|GetWidget) "NoCollision"))

(fn ShowContextMenu
  (bind _ascontext_menu_bp (CallFunction|GetContextMenu))
  (Default|OnShown _ascontext_menu_bp)
  (Variables|Default|SetWidgetShown true)
  (Collision|SetCollisionEnabled (Variables|Default|GetWidget) "QueryAndPhysics"))

(fn StopMoving
  (CallFunction|HideContextMenu)
  (bind _returnvalue (Class|ConstructableBuilding|StopMoving))
  (if (not _returnvalue)
    (bind _budgetcontroller (CallFunction|GetBudgetController))
    (Class|BudgetController|AddCurrency _budgetcontroller (.base_price (Class|ConstructableBuilding|GetInfo)))))

(fn GetContextMenu
  (bind _ascontext_menu_bp (Utilities|Casting|CastToContextMenu_BP (UserInterface|GetUserWidgetObject (Variables|Default|GetWidget))))
  (return _ascontext_menu_bp))

(fn ToggleContextMenu
  (params (Key :type Key%20Structure :default "None") (Actor :type Actor%20Object%20Reference))
  (if (Math|Boolean|ANDBoolean (== Key "RightMouseButton") (== (Actor|GetParentActor Actor) self) (Utilities|Enum|Equal(Enum) (Class|ConstructableBuilding|GetState) "Idle") (not (Variables|Default|GetWidgetShown)))
    (CallFunction|ShowContextMenu)
    (Transformation|SetWorldLocation (Variables|Default|GetWidget) (.WorldLocation (Game|Player|ConvertMouseLocationToWorldSpace (Game|GetPlayerController 0))) false false)
    (else
      (CallFunction|HideContextMenu))))

(fn CreateDetailsWidget
  (bind _returnvalue (UserInterface|CreateWidget "/Game/StableContent/UI/ContextMenu/Properties/BuildingDetails.BuildingDetails_C" (Game|GetPlayerController 0)))
  (bind _data (Default|GetBuildingInfo (Variables|Default|GetBuildingActor) self))
  (Default|InitializeBuilding _returnvalue (Class|ConstructableBuilding|GetInfo) _data)
  (return _returnvalue))

(event MouseInput|EventActorOnClicked
  (params (ButtonPressed :type Key%20Structure))
  ;[1 1 1] Click on building
  (CallFunction|ToggleContextMenu ButtonPressed self))

(event Input|MouseEvents|RightMouseButton
  (params (Key :type Key%20Structure))
  ;[1 1 1] Click on building
  (:Pressed
    (Development|PrintString (Utilities|GetObjectName self)))
  (:Released
    (bind _actor (CallFunction|GetActorUnderMousePointer))
    (bind _asbuilding_actor (Utilities|Casting|CastToBuildingActor _actor))
    (CallFunction|ToggleContextMenu Key _asbuilding_actor)))

(event Input|MouseEvents|LeftMouseButton
  (params (Key :type Key%20Structure))
  ;[1 1 1] Outer click & finish moving
  (:Released
    (CallFunction|StopMoving)
    (if (Variables|Default|GetWidgetShown)
      (CallFunction|HideContextMenu))))

(event EventSetInfo
  (params (info :type Building%20Settings%20Structure%20%28by%20ref%29))
  (|CallParentFunction info)
  (CallFunction|CreateBuilding)
  (Utilities|CreateContextMenu))

(event EventSetBuildingColor
  (params (Material :type BuildingColor%20Enum%20%28by%20ref%29 :default "Color_Normal"))
  (CallFunction|SetBuildingColor Material))